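; BP_Player is the player Character, with axis-driven movement, mouse look, jumping and an air dash.
; Movement follows the capsule's forward and right vectors, while mouse axes feed controller yaw and pitch.
; Each jump press calls Jump and increments a counter that triggers Dash at a count of two and resets on landing.
; Dash uses LaunchCharacter to add an upward boost plus a push along the current movement input.
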(event `InputAxis|Vertical`
  (params (AxisValue :type "Float (single-precision)"))
  ;[1 1 1] Movement System
  (`self.AddMovementInput` (`SceneComponent.GetForwardVector` (`self.CapsuleComponent`)) AxisValue))

(event `InputAxis|Mouse X`
  (params (AxisValue :type "Float (single-precision)"))
  ;[1 1 1] Rotation
  (`self.AddControllerYawInput` AxisValue))

(event `InputAxis|Mouse Y`
  (params (AxisValue :type "Float (single-precision)"))
  ;[1 1 1] Rotation
  (`self.AddControllerPitchInput` AxisValue))

(event `InputAxis|Horizontal`
  (params (AxisValue :type "Float (single-precision)"))
  ;[1 1 1] Movement System
  (`self.AddMovementInput` (`SceneComponent.GetRightVector` (`self.CapsuleComponent`)) AxisValue))

(event `InputAction|Jump`
  (params (Key :type "Key Structure"))
  ;[1 1 1] Jumping
  (:`Pressed`
    (`self.Jump`)
    (bind _result (`/Engine/EditorBlueprintResources/StandardMacros.IncrementInt` (`self.jumpedTimes`))
      (:`  `
        (switch `int` _result
          (:`2`
            (`self.Dash` 500.0)))))))

(event `self.OnLanded`
  (params (Hit :type "HitResult Structure (by ref)"))
  ;[1 1 1] Jumping
  (set `self.jumpedTimes` 0))

(fn `Dash`
  (params (DashForce :type "Float (double-precision)"))
  (bind _capsulecomponent (`self.CapsuleComponent`))
  (`self.LaunchCharacter` (+ (* (`SceneComponent.GetUpVector` _capsulecomponent) 300.0) (* (+ (* (`SceneComponent.GetRightVector` _capsulecomponent) (`self.GetInputAxisValue`)) (* (`SceneComponent.GetForwardVector` _capsulecomponent) (`self.GetInputAxisValue`))) DashForce))))

(fn `UserConstructionScript`)